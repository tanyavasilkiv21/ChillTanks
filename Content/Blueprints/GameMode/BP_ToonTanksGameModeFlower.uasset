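; Game mode Blueprint for a Toon Tanks level that handles the UI and audio at game start and game over.
; StartGame adds an audio component and puts the start, health and player point widgets on screen.
; GameOver stops that audio, adds an audio component for the win or loss, and shows the result widget and mouse cursor.
; It then removes the health and point widgets.
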(event `self.ReceiveTick`
  (params (DeltaSeconds :type "Float (single-precision)")))

(event `self.StartGame`
  (bind _returnvalue (`AddComponent|NODE_AddAudioComponent-3`))
  (bind _returnvalue_2 (`|CreateWidget` "/Game/Blueprints/Widgets/WBP_StartGameWidget.WBP_StartGameWidget_C"))
  (`UserWidget.AddToViewport` _returnvalue_2 0)
  (bind _returnvalue_3 (`|CreateWidget` "/Game/Blueprints/Widgets/WBP_HealthWidget.WBP_HealthWidget_C"))
  (`UserWidget.AddToViewport` _returnvalue_3 0)
  (bind _returnvalue_4 (`|CreateWidget` "/Game/Blueprints/Widgets/WBP_PlayerPointWidget.WBP_PlayerPointWidget_C"))
  (`UserWidget.AddToViewport` _returnvalue_4 0))

(event `self.GameOver`
  (params (bWonGame :type Boolean))
  (`AudioComponent.Stop` (stale `self.StartGame` _returnvalue))
  (if bWonGame
    (`AddComponent|NODE_AddAudioComponent-2`)
    (else
      (`AddComponent|NODE_AddAudioComponent-1`)))
  (bind _returnvalue (`|CreateWidget` "/Game/Blueprints/Widgets/WBP_GameOverWidget.WBP_GameOverWidget_C"))
  (`UserWidget.AddToViewport` _returnvalue 0)
  (set `PlayerController.bShowMouseCursor` true (`GameplayStatics.GetPlayerController` 0))
  (set `TextBlock.Text` (select `bool` bWonGame :`false` "Game Over!" :`true` "You Won!" :!type "Text") (`/Game/Blueprints/Widgets/WBP_GameOverWidget.DisplayText` _returnvalue))
  (`Widget.RemoveFromParent` (stale `self.StartGame` _returnvalue_3))
  (`Widget.RemoveFromParent` (stale `self.StartGame` _returnvalue_4)))

(fn `UserConstructionScript`)